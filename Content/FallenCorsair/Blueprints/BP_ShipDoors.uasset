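; Sliding double ship door in FallenCorsair that opens on sphere overlap once unlocked and closes when the overlap ends.
; A vector timeline slides LDoor and RDoor in mirrored directions, reversing on exit.
; The overlap is not filtered by actor type.
; MakeOpenable sets CanOpen, prints a debug "Hello", and flags both doors' dynamic materials through a CanOpen scalar parameter.
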(event `self.Sphere.OnComponentBeginOverlap`
  (params (OverlappedComponent :type "PrimitiveComponent Object Reference") (OtherActor :type "Actor Object Reference") (OtherComp :type "PrimitiveComponent Object Reference") (OtherBodyIndex :type Integer) (bFromSweep :type Boolean) (SweepResult :type "HitResult Structure (by ref)"))
  (if (`self.CanOpen`)
    (bind (_direction _newtrack_0) (`Timeline|Timeline` :!label _label)
      (:`Update`
        (`|ExecutionSequence`
          (:`then_0`
            (`SceneComponent.K2_SetRelativeLocation` (`self.RDoor`) (- (0.0 0.0 0.0) _newtrack_0) false false))
          (:`then_1`
            (`SceneComponent.K2_SetRelativeLocation` (`self.LDoor`) _newtrack_0 false false)))))))

(event `self.Sphere.OnComponentEndOverlap`
  (params (OverlappedComponent :type "PrimitiveComponent Object Reference") (OtherActor :type "Actor Object Reference") (OtherComp :type "PrimitiveComponent Object Reference") (OtherBodyIndex :type Integer))
  (goto _label :!via `Reverse`))

(fn `MakeOpenable`
  (set `self.CanOpen` true)
  (`KismetSystemLibrary.PrintText` "Hello")
  (bind _returnvalue (`PrimitiveComponent.CreateDynamicMaterialInstance` (`self.LDoor`) 1 null "None"))
  (`MaterialInstanceDynamic.SetScalarParameterValue` _returnvalue "CanOpen" 1.0)
  (bind _returnvalue_2 (`PrimitiveComponent.CreateDynamicMaterialInstance` (`self.RDoor`) 1 null "None"))
  (`MaterialInstanceDynamic.SetScalarParameterValue` _returnvalue_2 "CanOpen" 1.0))

(fn `UserConstructionScript`)