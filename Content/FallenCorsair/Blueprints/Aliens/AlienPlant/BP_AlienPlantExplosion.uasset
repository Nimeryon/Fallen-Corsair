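; Blueprint for an exploding alien plant, handling only its health bar display.
; On BeginPlay it caches the W_HP widget from the CWHP widget component.
; Each Tick it pushes current and max health, truncated to integers, into that widget.
; It also rotates the component along the horizontal direction from the owner to the player pawn, so the bar faces the player.
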(event `self.ReceiveBeginPlay`
  (bind _asw_hp (cast `/Game/FallenCorsair/Widgets/W_HP` (`WidgetComponent.GetWidget` (`self.CW_HP`))))
  (set `self.WidgetHp` _asw_hp))

(event `self.ReceiveTick`
  (params (DeltaSeconds :type "Float (single-precision)"))
  (if (`KismetSystemLibrary.IsValid` (`self.WidgetHp`))
    (`/Game/FallenCorsair/Widgets/W_HP.Set Hp` (`self.WidgetHp`) (`KismetMathLibrary.FTrunc` (`self.m_currentHealth`)) (`KismetMathLibrary.FTrunc` (`self.m_health`)))
    (`SceneComponent.K2_SetWorldRotation` (`self.CW_HP`) (`KismetMathLibrary.Conv_VectorToRotator` (`KismetMathLibrary.Vector_Normal2D` (- (`self.K2_GetActorLocation` (`GameplayStatics.GetPlayerPawn` 0)) (`self.K2_GetActorLocation` (`self.GetOwner`))))) false false)))

(fn `UserConstructionScript`)