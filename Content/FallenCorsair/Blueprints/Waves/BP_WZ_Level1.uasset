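; Wave zone for Level 1 that handles what happens when the zone's victory condition is met.
; On victory it zeroes the wave tracker's enemy limits, makes the exit door openable and plays the Level 01 end sequence.
; The sequence disables movement and look input and hides the HUD.
; Its play and finish callbacks switch player damage off for the cinematic and back on afterward.
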(event `self.VictoryConditionBase.OnZoneVictory`
  (bind _m_wavetracker (`self.m_waveTracker`))
  (set `WaveTracker.m_maxEnemies` 0 _m_wavetracker)
  (set `WaveTracker.m_minEnemies` 0 _m_wavetracker)
  (bind (_outactor _returnvalue) (`LevelSequencePlayer.CreateLevelSequencePlayer` "/Game/FallenCorsair/Sequencer/Sequencer_Level01_End.Sequencer_Level01_End" (make `MovieSceneSequencePlaybackSettings` false (struct) 1.0 0.0 false false true true false true)))
  (add `MovieSceneSequencePlayer.OnPlay` _returnvalue (delegate `OnPlay_Event`))
  (add `MovieSceneSequencePlayer.OnFinished` _returnvalue (delegate `OnFinished_Event`))
  (`/Game/FallenCorsair/Blueprints/BP_ShipDoors.MakeOpenable` (`self.OpenDoor`))
  (`MovieSceneSequencePlayer.Play` (`LevelSequenceActor.SequencePlayer` _outactor)))

(event `OnPlay_Event`
  (bind _asfallen_corsair_character (cast `FallenCorsairCharacter` (`GameplayStatics.GetPlayerPawn` 0)))
  (set `Actor.bCanBeDamaged` false _asfallen_corsair_character))

(event `OnFinished_Event`
  (bind _asfallen_corsair_character (cast `FallenCorsairCharacter` (`GameplayStatics.GetPlayerPawn` 0)))
  (set `Actor.bCanBeDamaged` true _asfallen_corsair_character))

(fn `UserConstructionScript`
  (`parent.UserConstructionScript`))