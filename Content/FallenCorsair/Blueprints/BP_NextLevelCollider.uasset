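; BP_NextLevelCollider is a trigger volume that moves the game on to a configured level when its box is overlapped.
; The first overlap, with no check on the overlapping actor, disables player input and fades the camera and audio out to a held full fade.
; After waiting one and a half times the fade duration, it re-enables input and opens the level by object reference.
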(event `self.Box.OnComponentBeginOverlap`
  (params (OverlappedComponent :type "PrimitiveComponent Object Reference") (OtherActor :type "Actor Object Reference") (OtherComp :type "PrimitiveComponent Object Reference") (OtherBodyIndex :type Integer) (bFromSweep :type Boolean) (SweepResult :type "HitResult Structure (by ref)"))
  (bind _fadeduration (`self.FadeDuration`))
  (`/Engine/EditorBlueprintResources/StandardMacros.DoOnce` false
    (:`Completed`
      (`self.DisableInput` (`GameplayStatics.GetPlayerCharacter` 0) (`GameplayStatics.GetPlayerController` 0))
      (`PlayerCameraManager.StartCameraFade` :`self` (`GameplayStatics.GetPlayerCameraManager` 0) :`ToAlpha` 1.0 :`Duration` (`self.FadeDuration`) :`bShouldFadeAudio` true :`bHoldWhenFinished` true)
      (`KismetSystemLibrary.Delay` (+ _fadeduration (/ _fadeduration 2.0)))
      (`self.EnableInput` (`GameplayStatics.GetPlayerCharacter` 0) (`GameplayStatics.GetPlayerController` 0))
      (`GameplayStatics.OpenLevelBySoftObjectPtr` (`self.Level`)))))

(fn `UserConstructionScript`)