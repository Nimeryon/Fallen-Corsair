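; Character melee combo component with two attack sets, chosen by how long input is held.
; Attack locks walking and rotation, then plays the current montage, whose notifies drive hits, owner lunges, swing sounds, combo chaining and recovery.
; Presses during an attack buffer the next hit, re-aimed along camera-relative move input.
; Hits box-trace pawns and launch characters with per-attack impulses, without applying damage; cancel input stops the montage and resets state.
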(event `EnhancedInput|/Game/ThirdPerson/Input/Actions/IA_Move`
  (params (ActionValue :type "Vector2D Structure") (ElapsedSeconds :type "Float (double-precision)") (TriggeredSeconds :type "Float (double-precision)") (InputAction :type "InputAction Object Reference" :default "/Game/ThirdPerson/Input/Actions/IA_Move.IA_Move"))
  (bind (_returnvalue_x _returnvalue_y) (`KismetMathLibrary.BreakVector` (`KismetMathLibrary.Conv_Vector2DToVector` ActionValue)))
  (:`Triggered`
    (if (`self.bCanAttack`)
      (set `self.Rotation` (`KismetMathLibrary.Conv_RotatorToVector` (`Actor.K2_GetActorRotation` (`self.Owner`))))
      (else
        (`self.CalculRotation` (`KismetMathLibrary.MakeVector` _returnvalue_y _returnvalue_x))))))

(event `Attack`
  (if (`self.bCanAttack`)
    (`self.FreezeRotation` true)
    (`self.EnableWalk` false)
    (set `self.bCanAttack` false)
    (`self.SetRotation` :!label _label)
    (bind _melee (`self.GetCurrentMelee`))
    (bind _notifyname (`|PlayMontage` (`Character.Mesh` (`self.Owner`)) (break `` _melee))
      (:`then`
        (set `self.CanExecuteNextAttack` true))
      (:`OnCompleted`
        (`self.ResetState` :!label _label_2)
        (set `self.bAttackStarted` false))
      (:`OnNotifyBegin`
        (switch `name` _notifyname
          (:`Hit`
            (`self.TriggerHit`)
            (`self.ResetVelocity`))
          (:`CanCombo`
            (bind _v (`self.Is Last Combo`))
            (if _v
              (`self.StartAttack` false)
              (elif (`self.ExecuteNextAttack`)
                (set `self.ExecuteNextAttack` false)
                (`self.IncrementCurrentAttack`)
                (goto _label))))
          (:`Recovery`
            (goto _label_2))
          (:`Propulsion`
            (`self.PropulseOwner`))
          (:`Hit_Soft`
            (`GameplayStatics.PlaySound2D` "/Game/Sound/Spear/Spear_Swing.Spear_Swing" 1.0 1.0 0.0 null null))
          (:`Hit_Fast`
            (`GameplayStatics.PlaySound2D` "/Game/Sound/Spear/Spear_Swing_Fast.Spear_Swing_Fast" 1.0 1.0 0.0 null null)))))
    (else
      (set `self.ExecuteNextAttack` (`self.CanExecuteNextAttack`)))))

(event `self.ReceiveBeginPlay`
  (bind _ascharacter (cast `Character` (`self.GetOwner`)))
  (set `self.Owner` _ascharacter))

(event `EnhancedInput|/Game/ThirdPerson/Input/Actions/IA_CancelMelee`
  (params (ActionValue :type Boolean) (ElapsedSeconds :type "Float (double-precision)") (TriggeredSeconds :type "Float (double-precision)") (InputAction :type "InputAction Object Reference" :default "/Game/ThirdPerson/Input/Actions/IA_CancelMelee.IA_CancelMelee"))
  (:`Started`
    (`self.CancelAttack`)))

(fn `AttackIsStarted`
  (returns (Started :type Boolean))
  (return (`self.bAttackStarted`)))

(fn `CalculRotation`
  (params (Rot :type "Vector Structure"))
  (bind _asbp_third_person_character (cast `/Game/ThirdPerson/Blueprints/BP_ThirdPersonCharacter` (`self.Owner`)))
  (set `self.Rotation` (`KismetMathLibrary.Vector_Normal2D` (`KismetMathLibrary.GreaterGreater_VectorRotator` Rot (`SpringArmComponent.GetTargetRotation` (`FallenCorsairCharacter.CameraBoom` _asbp_third_person_character))))))

(fn `CancelAttack`
  (bind _melee (`self.GetCurrentMelee`))
  (`AnimInstance.Montage_Stop` (`SkeletalMeshComponent.GetAnimInstance` (`Character.Mesh` (`self.Owner`))) 0.0 (break `` _melee))
  (`self.ResetState`))

(fn `EnableWalk`
  (params (Enable :type Boolean))
  (bind _charactermovement (`Character.CharacterMovement` (`self.Owner`)))
  (if Enable
    (set `CharacterMovementComponent.MaxWalkSpeed` 500.0 _charactermovement)
    (else
      (set `CharacterMovementComponent.MaxWalkSpeed` 0.0 _charactermovement))))

(fn `FreezeRotation`
  (params (Freeze :type Boolean))
  (bind _returnvalue (not Freeze))
  (bind _charactermovement (`Character.CharacterMovement` (`self.Owner`)))
  (set `CharacterMovementComponent.bUseControllerDesiredRotation` _returnvalue _charactermovement)
  (set `CharacterMovementComponent.bOrientRotationToMovement` _returnvalue _charactermovement))

(fn `GetCurrentMelee`
  (returns (Melee :type " Structure"))
  (bind _indexcurrentattack (`self.IndexCurrentAttack`))
  (switch `|SwitchEnum` (`self.TypeAttack`)
    (:`NewEnumerator0`
      (return (`|GetArrayItem` :`Dimension 1` _indexcurrentattack)))
    (:`NewEnumerator1`
      (return (`|GetArrayItem` :`Dimension 1` _indexcurrentattack)))))

(fn `IncrementCurrentAttack`
  (returns (IndexCurrentAttack :type Integer))
  (bind _output_get (set `self.IndexCurrentAttack` (mod (+ (`self.IndexCurrentAttack`) 1) (`KismetArrayLibrary.Array_Length` _))))
  (return _output_get))

(fn `Is Last Combo`
  (returns (v :type Boolean))
  (bind _indexcurrentattack (`self.IndexCurrentAttack`))
  (switch `|SwitchEnum` (`self.TypeAttack`)
    (:`NewEnumerator0`
      (return (== _indexcurrentattack (- (`KismetArrayLibrary.Array_Length` _) 1))))
    (:`NewEnumerator1`
      (return (== _indexcurrentattack (- (`KismetArrayLibrary.Array_Length` _) 1))))))

(fn `PropulseOwner`
  (params (NewParam :type " Structure"))
  (bind _owner (`self.Owner`))
  (bind _melee (`self.GetCurrentMelee`))
  (`CharacterMovementComponent.AddImpulse` (`Character.CharacterMovement` _owner) (* (`Actor.GetActorForwardVector` _owner) (break `` _melee)) true))

(fn `ResetCombo`
  (set `self.IndexCurrentAttack` 0)
  (set `self.bCanAttack` true))

(fn `ResetState`
  (`self.ResetCombo`)
  (`self.FreezeRotation` false)
  (`self.EnableWalk` true))

(fn `ResetVelocity`
  (set `MovementComponent.Velocity` (0.0 0.0 0.0) (`Character.CharacterMovement` (`self.Owner`))))

(fn `SetReleased`
  (params (Released :type Boolean))
  (set `self.Released` Released))

(fn `SetRotation`
  (`Actor.K2_SetActorRotation` (`self.Owner`) (`KismetMathLibrary.Conv_VectorToRotator` (`self.Rotation`)) false))

(fn `SetTypeAttack`
  (params (TypeAttack :type Byte :default 0))
  (if (not (`self.bAttackStarted`))
    (set `self.TypeAttack` TypeAttack)))

(fn `StartAttack`
  (params (Start :type Boolean))
  (if (`self.Released`)
    (set `self.bAttackStarted` Start)
    (if (== (`self.IndexCurrentAttack`) 0)
      (`self.Attack`)
      (`self.SetReleased` false))))

(fn `TriggerHit`
  (bind _owner (`self.Owner`))
  (bind _returnvalue (`Actor.GetActorForwardVector` _owner))
  (bind _melee (`self.GetCurrentMelee`))
  (bind _returnvalue_2 (+ (`Actor.K2_GetActorLocation` _owner) (* _returnvalue (.x (`.BoxOffset_48_F28188894F0E58D74EEB11A85DCCE6F6` (break `` _melee)))) (* (.y (`.BoxOffset_48_F28188894F0E58D74EEB11A85DCCE6F6` (break `` _melee))) (`Actor.GetActorRightVector` _owner)) (* (.z (`.BoxOffset_48_F28188894F0E58D74EEB11A85DCCE6F6` (break `` _melee))) (`Actor.GetActorUpVector` _owner))))
  (bind _outhits (`KismetSystemLibrary.BoxTraceMultiForObjects` :`Start` _returnvalue_2 :`End` _returnvalue_2 :`HalfSize` (break `` _melee) :`Orientation` (`KismetMathLibrary.Conv_VectorToRotator` _returnvalue) :`ObjectTypes` (`|MakeArray` "ObjectTypeQuery3" :!type "EObjectTypeQuery Enum") :`DrawDebugType` "ForDuration" :`DrawTime` 1.0))
  (for _array_element _outhits
    (bind _ascharacter (cast `Character` (`.HitActor` (`GameplayStatics.BreakHitResult` _array_element))))
    (bind (_returnvalue_x _returnvalue_y) (`KismetMathLibrary.BreakVector` (* _returnvalue (`.PropulsionForceForwardEnnemie_39_33815B014B5F3C15BC0D0D8B0ABEEB91` (break `` _melee)))))
    (`CharacterMovementComponent.AddImpulse` (`Character.CharacterMovement` _ascharacter) (`KismetMathLibrary.MakeVector` _returnvalue_x _returnvalue_y (`.PropulsionForceUpEnnemie_38_0C5D4D6C4EF0C87B9DFF6BAD3C730BA8` (break `` _melee))) true)))

(fn `UpdateTypeAttack`
  (params (ElapsedSeconds :type "Float (double-precision)"))
  (bind _started (`self.AttackIsStarted`))
  (if _started
    _
    (elif (< ElapsedSeconds (`self.DelayInputDepth`))
      (`self.SetTypeAttack` 0)
      (else
        (`self.SetTypeAttack` 0)
        (`self.StartAttack` true)))))