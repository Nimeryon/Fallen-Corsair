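; Placeholder enemy actor that stands in for a real enemy in the Fallen Corsair game mode's wave system.
; On BeginPlay it increments the wave manager's living-enemy count and gives itself a random lifespan of a few seconds.
; Tick slides it along the X axis at its Speed.
; When destroyed, it decrements the count and has the wave manager check how many enemies are left.
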(event `self.ReceiveBeginPlay`
  (bind _asbp_fallen_corsair_game_mode_kevin (cast `/Game/ProtoKevin/BP_FallenCorsairGameModeKevin` (`GameplayStatics.GetGameMode`)))
  (`/Engine/EditorBlueprintResources/StandardMacros.IncrementInt` (`/Game/ProtoKevin/BC_WaveManager.enemiesAlive` (`/Game/ProtoKevin/BP_FallenCorsairGameModeKevin.BC_WaveManager` _asbp_fallen_corsair_game_mode_kevin))
    (:`  `
      (`self.SetLifeSpan` (`KismetMathLibrary.RandomFloatInRange` 5.0 15.0)))))

(event `self.ReceiveTick`
  (params (DeltaSeconds :type "Float (single-precision)"))
  (bind _returnvalue_location (`KismetMathLibrary.BreakTransform` (`self.GetTransform`)))
  (`self.K2_SetActorRelativeTransform` (`KismetMathLibrary.MakeTransform` (+ (`KismetMathLibrary.MakeVector` (* DeltaSeconds (`self.Speed`))) _returnvalue_location))))

(event `self.ReceiveDestroyed`
  (bind _asbp_fallen_corsair_game_mode_kevin (cast `/Game/ProtoKevin/BP_FallenCorsairGameModeKevin` (`GameplayStatics.GetGameMode`)))
  (bind _bc_wavemanager (`/Game/ProtoKevin/BP_FallenCorsairGameModeKevin.BC_WaveManager` _asbp_fallen_corsair_game_mode_kevin))
  (`/Engine/EditorBlueprintResources/StandardMacros.DecrementInt` (`/Game/ProtoKevin/BC_WaveManager.enemiesAlive` _bc_wavemanager)
    (:`  `
      (`/Game/ProtoKevin/BC_WaveManager.CheckEnemyLeft` _bc_wavemanager))))

(fn `UserConstructionScript`)