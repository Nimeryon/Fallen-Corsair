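; BP_KitchenDoors is a sliding double door that locks behind an actor passing through and starts a wave zone.
; One timeline moves both panels in mirrored directions, opening on BeginPlay or sphere overlap while CanOpen is true.
; Overlap end always reverses it; exiting on the lower world-Y side also clears CanOpen and activates the linked wave zone, which BeginPlay deactivates.
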(event `self.ReceiveBeginPlay`
  (set `WaveZone.m_bIsActive` false (`self.activateWavezoneOnClose`))
  (if (`self.CanOpen`) :!label _label
    (bind (_direction _newtrack_0) (`Timeline|Timeline` :!label _label_2)
      (:`Update`
        (`|ExecutionSequence`
          (:`then_0`
            (`SceneComponent.K2_SetRelativeLocation` (`self.RDoor`) (- (0.0 0.0 0.0) _newtrack_0) false false))
          (:`then_1`
            (`SceneComponent.K2_SetRelativeLocation` (`self.LDoor`) _newtrack_0 false false)))))))

(event `self.Sphere.OnComponentBeginOverlap`
  (params (OverlappedComponent :type "PrimitiveComponent Object Reference") (OtherActor :type "Actor Object Reference") (OtherComp :type "PrimitiveComponent Object Reference") (OtherBodyIndex :type Integer) (bFromSweep :type Boolean) (SweepResult :type "HitResult Structure (by ref)"))
  (goto _label))

(event `self.Sphere.OnComponentEndOverlap`
  (params (OverlappedComponent :type "PrimitiveComponent Object Reference") (OtherActor :type "Actor Object Reference") (OtherComp :type "PrimitiveComponent Object Reference") (OtherBodyIndex :type Integer))
  (bind (_returnvalue_x _returnvalue_y) (`KismetMathLibrary.BreakVector` (`self.K2_GetActorLocation` OtherActor)))
  (bind (_returnvalue_x_2 _returnvalue_y_2) (`KismetMathLibrary.BreakVector` (`SceneComponent.K2_GetComponentLocation` (`self.DefaultSceneRoot`))))
  (if (< _returnvalue_y _returnvalue_y_2)
    (set `self.CanOpen` false)
    (set `WaveZone.m_bIsActive` true (`self.activateWavezoneOnClose`))
    (goto _label_2 :!via `Reverse`)
    (else
      (goto _label_2 :!via `Reverse`))))

(fn `UserConstructionScript`)