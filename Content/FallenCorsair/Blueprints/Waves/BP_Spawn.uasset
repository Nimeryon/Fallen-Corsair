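; BP_Spawn is a wave spawn point that configures its WaveSpawner and links it to a nearby WaveZone.
; The construction script applies DetectionRadius to both the spawner's distance-from-player setting and the Sphere's radius.
; It then runs a sphere overlap at that radius and assigns the first WaveZone found as the spawner's owning zone.
; The event graph holds no active logic.
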(fn `UserConstructionScript`
  (bind _detectionradius (`self.DetectionRadius`))
  (set `WaveSpawner.m_distanceFromPlayer` _detectionradius (`self.WaveSpawner`))
  (`SphereComponent.SetSphereRadius` (`self.Sphere`) _detectionradius false)
  (bind (_outactors _returnvalue) (`KismetSystemLibrary.SphereOverlapActors` (`self.K2_GetActorLocation`) _detectionradius (`|MakeArray` "ObjectTypeQuery1" "ObjectTypeQuery2" "ObjectTypeQuery3" "ObjectTypeQuery4" "ObjectTypeQuery5" "ObjectTypeQuery6" :!type "EObjectTypeQuery Enum") "/Script/FallenCorsair.WaveZone"))
  (if _returnvalue
    (bind _aswave_zone (cast `WaveZone` (`|GetArrayItem` _outactors)))
    (set `WaveSpawner.m_waveZoneOwner` _aswave_zone (`self.WaveSpawner`))))