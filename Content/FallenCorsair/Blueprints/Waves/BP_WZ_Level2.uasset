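; BP_WZ_Level2 is the Level 2 wave zone logic, tying alien inhibitor deaths to zone victory.
; On BeginPlay it binds to the death event of every BP_AlienInhibitor in the world and forwards deaths to VictoryConditionBase.
; When that component signals victory, it prints a message, zeroes the wave tracker's enemy limits, opens the door and moves the exit to a fixed height.
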(event `self.ReceiveBeginPlay`
  (bind _outactors (`GameplayStatics.GetAllActorsOfClass` "/Game/FallenCorsair/Blueprints/Aliens/AlienInhibitor/BP_AlienInhibitor.BP_AlienInhibitor_C"))
  (for _array_element _outactors
    (add `AlienBase.OnDeath` _array_element (delegate `OnDeath`))))

(event `OnDeath`
  (`VictoryConditionBase.OnEnemyDeath` (`self.VictoryConditionBase`) (stale `self.ReceiveBeginPlay` _array_element)))

(event `self.VictoryConditionBase.OnZoneVictory`
  (bind _m_wavetracker (`self.m_waveTracker`))
  (bind _exit (`self.exit`))
  (bind (_x _y) (`KismetMathLibrary.BreakVector3f` (`self.K2_GetActorLocation` _exit)))
  (`KismetSystemLibrary.PrintText` "Victory!")
  (set `WaveTracker.m_maxEnemies` 0 _m_wavetracker)
  (set `WaveTracker.m_minEnemies` 0 _m_wavetracker)
  (`/Game/FallenCorsair/Blueprints/BP_AlienDoor.open` (`self.door`))
  (`self.K2_SetActorLocation` _exit (`KismetMathLibrary.MakeVector` _x _y 300.0) false false))

(fn `UserConstructionScript`
  (`parent.UserConstructionScript`))