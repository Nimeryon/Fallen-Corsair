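; Actor component that shows the owning actor's distance from the player on a W_DistanceFromPlayer widget.
; InitWDFP caches the supplied widget component and its cast widget.
; UpdateWidgetDistanceFromPlayer writes the rounded distance in world units and turns the widget toward the player pawn using a 2D-normalized direction, keeping it upright.
; BeginPlay and Tick are unused, so both functions rely on external calls.
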(fn `InitW_DFP`
  (params (w_DFP :type "WidgetComponent Object Reference"))
  (bind _output_get (set `self.C_W_DFP` w_DFP))
  (bind _asw_distance_from_player (cast `/Game/Widgets/W_DistanceFromPlayer` (`WidgetComponent.GetWidget` _output_get)))
  (set `self.W_DFP` _asw_distance_from_player))

(fn `UpdateWidgetDistanceFromPlayer`
  (if (`KismetSystemLibrary.IsValid` (`self.W_DFP`))
    (`/Game/Widgets/W_DistanceFromPlayer.SetText` (`self.W_DFP`) (`KismetTextLibrary.Conv_Int64ToText` (`KismetMathLibrary.Round64` (`KismetMathLibrary.Vector_Distance` (`Actor.K2_GetActorLocation` (`GameplayStatics.GetPlayerPawn` 0)) (`Actor.K2_GetActorLocation` (`self.GetOwner`))))))
    (`SceneComponent.K2_SetWorldRotation` (`self.C_W_DFP`) (`KismetMathLibrary.Conv_VectorToRotator` (`KismetMathLibrary.Vector_Normal2D` (- (`Actor.K2_GetActorLocation` (`GameplayStatics.GetPlayerPawn` 0)) (`Actor.K2_GetActorLocation` (`self.GetOwner`))))) false false)))