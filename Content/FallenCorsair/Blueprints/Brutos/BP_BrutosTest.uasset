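; BP_BrutosTest is a test Blueprint for Brutos that exercises camera-proximity fading and a low-HP post-process toggle.
; Each Tick maps the distance from FollowCamera to the actor onto the BrutosTest materials' Opacity, fading it out as the camera closes in.
; The A key flip-flops bIsLowHP in the MPC_PP parameter collection.
; BeginPlay stores a dynamic material instance in Mat, which the graph never uses afterwards.
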(event `Key|A`
  (params (Key :type "Key Structure"))
  (:`Pressed`
    (`/Engine/EditorBlueprintResources/StandardMacros.FlipFlop`
      (:`A`
        (`KismetMaterialLibrary.SetScalarParameterValue` "/Game/FallenCorsair/Blueprints/Brutos/MPC_PP.MPC_PP" "bIsLowHP" 1.0))
      (:`B`
        (`KismetMaterialLibrary.SetScalarParameterValue` "/Game/FallenCorsair/Blueprints/Brutos/MPC_PP.MPC_PP" "bIsLowHP")))))

(event `self.ReceiveBeginPlay`
  (bind _returnvalue (`KismetMaterialLibrary.CreateDynamicMaterialInstance` null))
  (set `self.Mat` _returnvalue))

(event `self.ReceiveTick`
  (params (DeltaSeconds :type "Float (single-precision)"))
  (`MeshComponent.SetScalarParameterValueOnMaterials` (`self.BrutosTest`) "Opacity" (`KismetMathLibrary.MapRangeClamped` (`KismetMathLibrary.Vector_Distance` (`SceneComponent.K2_GetComponentLocation` (`self.FollowCamera`)) (`self.K2_GetActorLocation`)) 80.0 160.0 0.0 1.0)))

(fn `UserConstructionScript`)