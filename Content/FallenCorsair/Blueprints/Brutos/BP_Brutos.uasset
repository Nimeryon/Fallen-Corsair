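; BP_Brutos is the Brutos actor Blueprint, with a follow camera and a viewfinder HUD.
; On BeginPlay it creates the W_Viewfinder widget and adds it to the viewport.
; Holding T slows global time to a crawl and holding G sets dilation to zero, with release restoring normal speed.
; The construction script positions FollowCamera from the OffsetCamera variable.
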(event `self.ReceiveBeginPlay`
  ;[1 1 1] Curseur
  (bind _returnvalue (`|CreateWidget` "/Game/FallenCorsair/Widgets/Viewfinder/W_Viewfinder.W_Viewfinder_C"))
  (`UserWidget.AddToViewport` _returnvalue 0))

(event `Key|T`
  (params (Key :type "Key Structure"))
  (:`Pressed`
    (`GameplayStatics.SetGlobalTimeDilation` 0.05))
  (:`Released`
    (`GameplayStatics.SetGlobalTimeDilation` 1.0)))

(event `Key|G`
  (params (Key :type "Key Structure"))
  (:`Pressed`
    (`GameplayStatics.SetGlobalTimeDilation` 0.0))
  (:`Released`
    (`GameplayStatics.SetGlobalTimeDilation` 1.0)))

(fn `UserConstructionScript`
  ;[1 1 1] Set The Offset Of The Camera
  (`SceneComponent.K2_SetRelativeLocation` (`self.FollowCamera`) (`self.OffsetCamera`) false false))