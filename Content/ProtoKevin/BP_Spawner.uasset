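; Spawner actor that places grounded alien AI at its own location for the wave system in the Kevin prototype game mode.
; The wave manager's WaveOver event re-arms it, with the same-zone check still a placeholder.
; Once active, Tick spawns batches after a random delay, or none with WaveEffect, capped by the manager's shared alive-enemy limit.
; The spawn counter checked against MaxSpawns only increments when SpawnIndefinitely is set.
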(event `self.ReceiveBeginPlay`
  (bind _asbp_fallen_corsair_game_mode_kevin (cast `/Game/ProtoKevin/BP_FallenCorsairGameModeKevin` (`GameplayStatics.GetGameMode`)))
  (add `/Game/ProtoKevin/BC_WaveManager.WaveOver` (`/Game/ProtoKevin/BP_FallenCorsairGameModeKevin.BC_WaveManager` _asbp_fallen_corsair_game_mode_kevin) (delegate `OnWaveOver`))
  (set `self.GameMode` _asbp_fallen_corsair_game_mode_kevin))

(event `OnWaveOver`
  (if (not false)
    (set `self.ShouldSpawn` true)))

(event `self.ReceiveTick`
  (params (DeltaSeconds :type "Float (single-precision)"))
  (bind _returnvalue_location (`KismetMathLibrary.BreakTransform` (`self.GetTransform`)))
  (bind _bc_wavemanager (`/Game/ProtoKevin/BP_FallenCorsairGameModeKevin.BC_WaveManager` (`self.GameMode`)))
  (bind _bc_wavemanager_2 (`/Game/ProtoKevin/BP_FallenCorsairGameModeKevin.BC_WaveManager` (`self.GameMode`)))
  (if (and (`self.IsActive`) (`self.ShouldSpawn`) (not (`self.IsSpawning`)) (!= (`self.NumberOfSpawns`) (`self.MaxSpawns`)) (>= (`self.GetGameTimeSinceCreation`) (`self.TimeToActivation`)))
    (set `self.IsSpawning` true)
    (bind _delay (`self.GetDelay`))
    (`KismetSystemLibrary.Delay` _delay)
    (for _ (range (+ (`KismetMathLibrary.Min` (`self.MinSpawn`) (- (`/Game/ProtoKevin/BC_WaveManager.maxEnemies` _bc_wavemanager) (`/Game/ProtoKevin/BC_WaveManager.enemiesAlive` _bc_wavemanager))) 1))
      (bind _returnvalue (`AIBlueprintHelperLibrary.SpawnAIFromClass` "/Game/FallenCorsair/Blueprints/Aliens/BP_GroundedAlien.BP_GroundedAlien_C" "/Game/FallenCorsair/AI/BehaviorThree/BT_GroundAlien.BT_GroundAlien" _returnvalue_location (struct) true null))
      (`/Engine/EditorBlueprintResources/StandardMacros.IsValid` _returnvalue
        (:`Is Valid`
          (`/Engine/EditorBlueprintResources/StandardMacros.IncrementInt` (`/Game/ProtoKevin/BC_WaveManager.enemiesAlive` (`/Game/ProtoKevin/BP_FallenCorsairGameModeKevin.BC_WaveManager` (`self.GameMode`)))))))
    (set `self.IsSpawning` false)
    (set `self.ShouldSpawn` (< (`/Game/ProtoKevin/BC_WaveManager.enemiesAlive` _bc_wavemanager_2) (`/Game/ProtoKevin/BC_WaveManager.maxEnemies` _bc_wavemanager_2)))
    (if (`self.SpawnIndefinitely`)
      (`/Engine/EditorBlueprintResources/StandardMacros.IncrementInt` (`self.NumberOfSpawns`)))))

(fn `GetDelay`
  (returns (Delay :type "Float (double-precision)"))
  (if (`self.WaveEffect`)
    (return 0.0)
    (else
      (return (`KismetMathLibrary.RandomFloatInRange` (`self.SpawnRateMin`) (`self.SpawnRateMax`))))))

(fn `UserConstructionScript`)